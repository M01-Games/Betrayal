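; BP_Photobook is a one-time interactable photo album that advances the Level 1 story.
; Player overlap with its sphere shows a press-F widget and enables input.
; Pressing F removes the prompt and album meshes, disables further interaction and shows a narrative comment through the first-person character.
; It then hands BP_AI_Mother new dialogue, an after-comment and a butler to spawn afterwards.
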(event OnComponentBeginOverlap(Sphere)
  (params (OverlappedComponent :type Primitive%20Component%20Object%20Reference) (OtherActor :type Actor%20Object%20Reference) (OtherComp :type Primitive%20Component%20Object%20Reference) (OtherBodyIndex :type Integer) (bFromSweep :type Boolean) (SweepResult :type Hit%20Result%20Structure%20%28by%20ref%29))
  ;[1 1 1] Enable Input
  (if (Actor|ActorHasTag OtherActor "Player")
    (bind _returnvalue (UserInterface|CreateWidget "/Game/BP/AI/WB_PressF.WB_PressF_C"))
    (UserInterface|Viewport|AddtoViewport _returnvalue 0)
    (Input|EnableInput (Game|GetPlayerController 0))))

(event OnComponentEndOverlap(Sphere)
  (params (OverlappedComponent :type Primitive%20Component%20Object%20Reference) (OtherActor :type Actor%20Object%20Reference) (OtherComp :type Primitive%20Component%20Object%20Reference) (OtherBodyIndex :type Integer))
  ;[1 1 1] Enable Input
  (if (Actor|ActorHasTag OtherActor "Player")
    (Utilities|IsValid (stale OnComponentBeginOverlap(Sphere) _returnvalue)
      (:Is%20Valid
        (Widget|RemovefromParent (stale OnComponentBeginOverlap(Sphere) _returnvalue))
        (Input|DisableInput (Game|GetPlayerController 0))))))

(event Input|KeyboardEvents|F
  (params (Key :type Key%20Structure :default "None"))
  (:Pressed
    (Utilities|FlowControl|DoOnce false
      (:Completed
        (Utilities|FlowControl|Sequence
          (:then_0
            ;[1 1 1] Enable Input
            (Widget|RemovefromParent (stale OnComponentBeginOverlap(Sphere) _returnvalue))
            (Input|DisableInput (Game|GetPlayerController 0)))
          (:then_1
            (Collision|SetCollisionEnabled (Variables|Default|GetSphere) "NoCollision")
            (Components|DestroyComponent (Variables|Default|GetCube1))
            (bind _returnvalue (Actor|GetActorOfClass "/Game/FirstPerson/Blueprints/BP_FirstPersonCharacter.BP_FirstPersonCharacter_C"))
            (Default|CallComment _returnvalue "You pick up the photo album and flip to the first page. You see you and father along with the rest of your family arranged in the living room for a photo shoot, only when you try and focus on you or your fathers face, you can’t seem to be able to, like it’s shrouded in a blur you can’t focus through. You close the photo album, you no longer want to have it anywhere near you. You take it to your mother." 15.0)
            (bind _returnvalue_2 (Actor|GetActorOfClass "/Game/BP/AI/BP_AI_Mother.BP_AI_Mother_C"))
            (Variables|/Game/BP/AI/BP_AI.BP_AI_C|SetDialogue _returnvalue_2 (Variables|Default|GetDialogue))
            (Variables|/Game/BP/AI/BP_AI.BP_AI_C|SetafterComment _returnvalue_2 true)
            (Variables|/Game/BP/AI/BP_AI.BP_AI_C|SetAfter%20CommentText _returnvalue_2 "Internal: *Sigh* I need a drink. I wonder if there's still whiskey is still in the library.")
            (Default|ResetSpawnDoOnce _returnvalue_2)
            (Variables|/Game/BP/AI/BP_AI.BP_AI_C|SetspawnAfter _returnvalue_2 true)
            (Variables|/Game/BP/AI/BP_AI.BP_AI_C|SetSpawn%20After%20Class _returnvalue_2 "/Game/BP/AI/BP_AI_Butler.BP_AI_Butler_C")
            (Variables|/Game/BP/AI/BP_AI.BP_AI_C|SetSpawnAfterLocation _returnvalue_2 "614.477389,1204.027676,99.431584")
            (Variables|/Game/BP/AI/BP_AI.BP_AI_C|SetSpawn%20After%20Rotation _returnvalue_2 "0.000000,39.104538,0.000000")))))))

(fn ConstructionScript)