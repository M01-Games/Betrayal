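; BP_SignificantDoor is a Level 1 door that teleports the player to a set location behind a black fade.
; Overlapping its box with the Player tag shows a press-F widget and enables input; leaving reverses both.
; F runs once through DoOnce, fading to black, moving the player character and fading back after delays.
; Optional flags then play a sound, stop BP_LevelOneManager's sounds or trigger a first-person character comment.
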(event OnComponentBeginOverlap(Box)
  (params (OverlappedComponent :type Primitive%20Component%20Object%20Reference) (OtherActor :type Actor%20Object%20Reference) (OtherComp :type Primitive%20Component%20Object%20Reference) (OtherBodyIndex :type Integer) (bFromSweep :type Boolean) (SweepResult :type Hit%20Result%20Structure%20%28by%20ref%29))
  ;[1 1 1] Enable Input
  (if (Actor|ActorHasTag OtherActor "Player")
    (bind _returnvalue (UserInterface|CreateWidget "/Game/BP/AI/WB_PressF.WB_PressF_C"))
    (UserInterface|Viewport|AddtoViewport _returnvalue 0)
    (Input|EnableInput (Game|GetPlayerController 0))))

(event OnComponentEndOverlap(Box)
  (params (OverlappedComponent :type Primitive%20Component%20Object%20Reference) (OtherActor :type Actor%20Object%20Reference) (OtherComp :type Primitive%20Component%20Object%20Reference) (OtherBodyIndex :type Integer))
  ;[1 1 1] Enable Input
  (if (Actor|ActorHasTag OtherActor "Player")
    (Widget|RemovefromParent (stale OnComponentBeginOverlap(Box) _returnvalue))
    (Input|DisableInput (Game|GetPlayerController 0))))

(event Input|KeyboardEvents|F
  (params (Key :type Key%20Structure :default "None"))
  ;[1 1 1] Fade in and Move
  (:Pressed
    (Utilities|FlowControl|DoOnce false
      (:Completed
        (bind _returnvalue (UserInterface|CreateWidget "/Game/FirstPerson/Blueprints/FadeInAndOut.FadeInAndOut_C"))
        (UserInterface|Viewport|AddtoViewport _returnvalue 0)
        (Default|BlackFadein _returnvalue)
        (Utilities|FlowControl|Delay 1.0)
        (Transformation|SetActorLocation (Game|GetPlayerCharacter 0) (Variables|Default|GetWhere%20to%20send%20Player) false false)
        (Utilities|FlowControl|Delay 1.0)
        (Default|BlackFadeOut _returnvalue)
        (if (Variables|Default|GetplaySoundOnTeleport)
          (Audio|PlaySound2D (Variables|Default|GetSoundToPlay) 0.8 1.0 0.0 0 0 false))
        (if (Variables|Default|GetstopSounds)
          (Utilities|FlowControl|Delay 0.5)
          (bind _returnvalue_2 (Actor|GetActorOfClass "/Game/GameLevels/Level1/BP_LevelOneManager.BP_LevelOneManager_C"))
          (Default|StopAllSound _returnvalue_2))
        (if (Variables|Default|GetsayComment)
          (bind _returnvalue_3 (Actor|GetActorOfClass "/Game/FirstPerson/Blueprints/BP_FirstPersonCharacter.BP_FirstPersonCharacter_C"))
          (Default|CallComment _returnvalue_3 (Variables|Default|GetComment)))))))

(fn ConstructionScript)