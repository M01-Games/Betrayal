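; Interactable knife actor that triggers an ending sequence when the player presses F near it.
; A sphere overlap with the Player-tagged actor shows the WB_PressF prompt and enables input, and leaving removes the prompt and calls DisableInput.
; The one-shot F press puts the knife in the character's hand, plays a wind sound and shows a despairing comment, then loads StartLevel after a delay.
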(event OnComponentBeginOverlap(Sphere)
  (params (OverlappedComponent :type Primitive%20Component%20Object%20Reference) (OtherActor :type Actor%20Object%20Reference) (OtherComp :type Primitive%20Component%20Object%20Reference) (OtherBodyIndex :type Integer) (bFromSweep :type Boolean) (SweepResult :type Hit%20Result%20Structure%20%28by%20ref%29))
  (if (Actor|ActorHasTag OtherActor "Player")
    (bind _returnvalue (UserInterface|CreateWidget "/Game/BP/AI/WB_PressF.WB_PressF_C"))
    (UserInterface|Viewport|AddtoViewport _returnvalue 0)
    (Input|EnableInput (Game|GetPlayerController 0))))

(event OnComponentEndOverlap(Sphere)
  (params (OverlappedComponent :type Primitive%20Component%20Object%20Reference) (OtherActor :type Actor%20Object%20Reference) (OtherComp :type Primitive%20Component%20Object%20Reference) (OtherBodyIndex :type Integer))
  (if (Actor|ActorHasTag OtherActor "Player")
    (Widget|RemovefromParent (stale OnComponentBeginOverlap(Sphere) _returnvalue))
    (Input|DisableInput (Game|GetPlayerController 0) 0)))

(event Input|KeyboardEvents|F
  (params (Key :type Key%20Structure :default "None"))
  (:Pressed
    (Utilities|FlowControl|DoOnce false
      (:Completed
        (bind _returnvalue (Actor|GetActorOfClass "/Game/FirstPerson/Blueprints/BP_FirstPersonCharacter.BP_FirstPersonCharacter_C"))
        (Default|SetKnifeinHand _returnvalue)
        (Audio|PlaySound2D "/Game/Sound/SFX_and_Ambience/Hallow_Wind.Hallow_Wind" 2.0 0.7 0.0 0 0)
        (bind _returnvalue_2 (Actor|GetActorOfClass "/Game/FirstPerson/Blueprints/BP_FirstPersonCharacter.BP_FirstPersonCharacter_C"))
        (Default|CallComment _returnvalue_2 "Oh no... it's happening again... 
What do I tell my family..." 5.0)
        (Utilities|FlowControl|Delay 8.0)
        (Game|OpenLevel(byObjectReference) "/Game/GameLevels/StartLevel.StartLevel")))))

(fn ConstructionScript)