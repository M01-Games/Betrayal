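; BP_AI_2 is a talkable AI character that shows a prompt widget while something overlaps its trigger zone.
; Each Communicate call advances a talk index through the Dialogue array, creating a WB_Dialogue widget if none is valid and setting its text to the current line.
; Once the lines run out, it removes the dialogue widget from the screen.
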(event OnComponentBeginOverlap(Trigger_Zone)
  (params (OverlappedComponent :type Primitive%20Component%20Object%20Reference) (OtherActor :type Actor%20Object%20Reference) (OtherComp :type Primitive%20Component%20Object%20Reference) (OtherBodyIndex :type Integer) (bFromSweep :type Boolean) (SweepResult :type Hit%20Result%20Structure%20%28by%20ref%29))
  ;[1 1 1] LOOK_AT_BELOW!
  (Rendering|SetVisibility (Variables|Default|GetWidget) true false))

(event OnComponentEndOverlap(Trigger_Zone)
  (params (OverlappedComponent :type Primitive%20Component%20Object%20Reference) (OtherActor :type Actor%20Object%20Reference) (OtherComp :type Primitive%20Component%20Object%20Reference) (OtherBodyIndex :type Integer))
  ;[1 1 1] LOOK_AT_BELOW!
  (Rendering|SetVisibility (Variables|Default|GetWidget) false false))

(event EventCommunicate
  ;[1 1 1] Communication_with_AI_Mechanic
  (Math|Integer|IncrementInt (Variables|Default|GetTalk_Index)
    (:%20%20
      (if (< (Variables|Default|GetTalk_Index) (Utilities|Array|Length (Variables|Default|GetDialogue)))
        (Variables|Default|GetUI
          (:then
            _)
          (:else
            (bind _returnvalue (UserInterface|CreateWidget "/Game/BP/AI/WB_Dialogue.WB_Dialogue_C" (Game|GetPlayerController 0)))
            (bind _output_get (Variables|Default|SetUI _returnvalue))
            (UserInterface|Viewport|AddtoViewport _output_get 0)))
        (Rendering|Components|TextRender|SetText (Variables|/Game/BP/AI/WB_Dialogue.WB_Dialogue_C|GetTalk_Text (Variables|Default|GetUI)) (Utilities|Text|ToText(String) (Utilities|Array|Get(acopy) (Variables|Default|GetDialogue) (Variables|Default|GetTalk_Index))))
        (else
          (Widget|RemovefromParent (Variables|Default|GetUI)))))))

(fn ConstructionScript)