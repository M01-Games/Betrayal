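; Interactable knife ending trigger that gives the player the knife and sends the game to StartLevel.
; Player overlap with the trigger zone shows a press-F widget and enables input, with paired DoOnce nodes toggling the prompt on enter and exit.
; Pressing F disables the zone's collision, calls SetKnifeInHand, plays a wind sound and loads the level after a delay.
; Leftover AI dialogue and spawn-after logic remains, largely unconnected.
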(event OnComponentBeginOverlap(Trigger_Zone)
  (params (OverlappedComponent :type Primitive%20Component%20Object%20Reference) (OtherActor :type Actor%20Object%20Reference) (OtherComp :type Primitive%20Component%20Object%20Reference) (OtherBodyIndex :type Integer) (bFromSweep :type Boolean) (SweepResult :type Hit%20Result%20Structure%20%28by%20ref%29))
  (bind _returnvalue (Game|GetPlayerController 0))
  ;[1 1 1] overlap triggers
  (if (Actor|ActorHasTag OtherActor "Player")
    (Utilities|FlowControl|Sequence
      (:then_0
        (Utilities|FlowControl|DoOnce false
          (:Completed
            (bind _returnvalue_2 (UserInterface|CreateWidget "/Game/BP/AI/WB_PressF.WB_PressF_C"))
            (UserInterface|Viewport|AddtoViewport _returnvalue_2 0)
            (Input|EnableInput _returnvalue))))
      (:then_1
        (Utilities|FlowControl|DoOnce false) ; enters at Reset
      ))))

(event OnComponentEndOverlap(Trigger_Zone)
  (params (OverlappedComponent :type Primitive%20Component%20Object%20Reference) (OtherActor :type Actor%20Object%20Reference) (OtherComp :type Primitive%20Component%20Object%20Reference) (OtherBodyIndex :type Integer))
  (bind _returnvalue (Game|GetPlayerController 0))
  ;[1 1 1] overlap triggers
  (if (Actor|ActorHasTag OtherActor "Player")
    (Utilities|FlowControl|Sequence
      (:then_0
        (Utilities|FlowControl|DoOnce false
          (:Completed
            (Widget|RemovefromParent (stale OnComponentBeginOverlap(Trigger_Zone) _returnvalue_2))
            (Input|DisableInput _returnvalue))))
      (:then_1
        (Utilities|FlowControl|DoOnce false) ; enters at Reset
      ))))

(event Custom|ResetSpawnDoOnce
  ;[1 1 1] Communication_with_AI_Mechanic
  (Utilities|FlowControl|DoOnce false) ; enters at Reset
)

(event Input|KeyboardEvents|F
  (params (Key :type Key%20Structure :default "None"))
  ;[1 1 1] Communication_with_AI_Mechanic
  (:Pressed
    (Collision|SetCollisionEnabled (Variables|Default|GetTrigger_Zone) "NoCollision")
    (Utilities|FlowControl|DoOnce false
      (:Completed
        (Development|PrintString "TEST")
        (bind _asbp_first_person_character (Utilities|Casting|CastToBP_FirstPersonCharacter (Game|GetPlayerCharacter 0)))
        (Default|SetKnifeinHand _asbp_first_person_character)
        (Audio|PlaySound2D "/Game/Sound/SFX_and_Ambience/Hallow_Wind.Hallow_Wind" 2.0 0.7 0.0 0 0)
        (Utilities|FlowControl|Delay 5.0)
        (Game|OpenLevel(byObjectReference) "/Game/GameLevels/StartLevel.StartLevel")))))

(fn ConstructionScript)